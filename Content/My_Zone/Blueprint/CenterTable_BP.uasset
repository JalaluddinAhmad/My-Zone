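; CenterTable_BP is a center table actor that animates its parts on BeginPlay and whenever its Table event is called.
; Both events restart one timeline, whose track drives lerps on three scene components.
; Scene slides in X and Z, Scene2 rotates, and Scene1 does both.
; The location endpoints are hardcoded, large-valued coordinates applied as relative locations, so the motion depends on that specific setup.
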(event `self.ReceiveBeginPlay`
  (bind (_direction _newtrack_0) (`Timeline|Timeline_0` :!via `PlayFromStart` :!label _label)
    (:`Update`
      (`SceneComponent.K2_SetRelativeLocation` (`self.Scene`) (`KismetMathLibrary.MakeVector` (`KismetMathLibrary.Lerp` -20745.919922 -20772.0 _newtrack_0) -3840.036133 (`KismetMathLibrary.Lerp` 48.229248 62.0 _newtrack_0)) false false)
      (`SceneComponent.K2_SetRelativeRotation` (`self.Scene2`) (`KismetMathLibrary.RLerp` (struct) (struct :`Pitch` 60.0) _newtrack_0) false false)
      (`SceneComponent.K2_SetRelativeLocationAndRotation` (`self.Scene1`) (`KismetMathLibrary.MakeVector` (`KismetMathLibrary.Lerp` -20745.919922 -20748.0 _newtrack_0) -3840.036133 (`KismetMathLibrary.Lerp` 38.0 44.06543 _newtrack_0)) (`KismetMathLibrary.RLerp` (struct) (struct :`Pitch` 100.0) _newtrack_0) false false))))

(event `Table`
  (goto _label :!via `PlayFromStart`))

(fn `UserConstructionScript`)