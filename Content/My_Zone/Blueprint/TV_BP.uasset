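; TV actor Blueprint that continuously swings its Scene component back and forth through a 180-degree rotation.
; On BeginPlay, Timeline_0 drives a rotator lerp forward, then Timeline_1 plays in reverse to lerp back.
; Each timeline's completion starts the other after a short delay, forming an endless loop.
; A custom TV event also starts the forward timeline from the beginning.
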(event `self.ReceiveBeginPlay`
  (bind (_direction _newtrack_0) (`Timeline|Timeline_0` :!via `PlayFromStart` :!label _label)
    (:`Update`
      (`SceneComponent.K2_SetRelativeRotation` (`self.Scene`) (`KismetMathLibrary.RLerp` (struct) (struct :`Yaw` 180.0) _newtrack_0) false false))
    (:`Finished`
      (`KismetSystemLibrary.Delay` 1.0)
      (bind (_direction_2 _newtrack_0_2) (`Timeline|Timeline_1` :!via `ReverseFromEnd`)
        (:`Update`
          (`SceneComponent.K2_SetRelativeRotation` (`self.Scene`) (`KismetMathLibrary.RLerp` (struct) (struct :`Yaw` 180.0) _newtrack_0_2) false false))
        (:`Finished`
          (`KismetSystemLibrary.Delay` 1.0)
          (goto _label :!via `PlayFromStart`))))))

(event `TV`
  (goto _label :!via `PlayFromStart`))

(fn `UserConstructionScript`)