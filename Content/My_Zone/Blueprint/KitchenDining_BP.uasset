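; Animated kitchen dining table that slides and rotates its parts into a second configuration and can reverse the motion.
; KitchenTable and BeginPlay both start Timeline_0, whose alpha drives lerps on three scene components and the table front mesh.
; ReverseKitchen plays a separate Timeline_1 backwards over similar lerps, but only rotates the Scene component without restoring its location.
; The forward timeline ends in a Delay with nothing after it.
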(event `KitchenTable`
  (bind (_direction _newtrack_0) (`Timeline|Timeline_0` :!via `PlayFromStart` :!label _label)
    (:`Update`
      (`SceneComponent.K2_SetRelativeLocationAndRotation` (`self.Scene1`) (`KismetMathLibrary.MakeVector` (`KismetMathLibrary.Lerp` -20627.703125 -20781.0 _newtrack_0) -3989.061523 76.0) (`KismetMathLibrary.RLerp` (struct) (struct :`Pitch` -90.0) _newtrack_0) false false)
      (`SceneComponent.K2_SetRelativeLocationAndRotation` (`self.Scene`) (`KismetMathLibrary.MakeVector` (`KismetMathLibrary.Lerp` -20524.0 -20617.388672 _newtrack_0) -3989.061523 76.0) (`KismetMathLibrary.RLerp` (struct) (struct :`Pitch` 90.0) _newtrack_0) false false)
      (`SceneComponent.K2_SetRelativeLocationAndRotation` (`self.Scene2`) (`KismetMathLibrary.MakeVector` (`KismetMathLibrary.Lerp` -20615.763672 -20699.0 _newtrack_0) -3989.061523 71.723541) (`KismetMathLibrary.RLerp` (struct) (struct :`Yaw` 90.0) _newtrack_0) false false)
      (`SceneComponent.K2_SetRelativeLocation` (`self.SM_Dinner_Table_Front`) (`KismetMathLibrary.MakeVector` (`KismetMathLibrary.Lerp` 0.0 -135.0 _newtrack_0)) false false))
    (:`Finished`
      (`KismetSystemLibrary.Delay` 2.0))))

(event `self.ReceiveBeginPlay`
  (goto _label :!via `PlayFromStart`))

(event `Reverse Kitchen`
  (bind (_direction _newtrack_0) (`Timeline|Timeline_1` :!via `ReverseFromEnd`)
    (:`Update`
      (`SceneComponent.K2_SetRelativeLocationAndRotation` (`self.Scene1`) (`KismetMathLibrary.MakeVector` (`KismetMathLibrary.Lerp` -20627.703125 -20781.0 _newtrack_0) -3989.061523 76.0) (`KismetMathLibrary.RLerp` (struct) (struct :`Pitch` -90.0) _newtrack_0) false false)
      (`SceneComponent.K2_SetRelativeRotation` (`self.Scene`) (`KismetMathLibrary.RLerp` (struct) (struct :`Pitch` 90.0) _newtrack_0) false false)
      (`SceneComponent.K2_SetRelativeLocationAndRotation` (`self.Scene2`) (`KismetMathLibrary.MakeVector` (`KismetMathLibrary.Lerp` -20615.763672 -20699.0 _newtrack_0) -3989.061523 71.723541) (`KismetMathLibrary.RLerp` (struct) (struct :`Yaw` 90.0) _newtrack_0) false false)
      (`SceneComponent.K2_SetRelativeLocation` (`self.SM_Dinner_Table_Front`) (`KismetMathLibrary.MakeVector` (`KismetMathLibrary.Lerp` 0.0 -135.0 _newtrack_0)) false false))))

(fn `UserConstructionScript`)